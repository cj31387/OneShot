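; AI character for a OneShot game that uses pawn sensing to chase pawns it has seen.
; OnSeePawn collects unique pawns, prints their names and updates ClosestPawn through a distance comparison.
; A self-calling AIRoam loop idles until ClosestPawn is valid, then repeatedly moves toward it while the sensing component's SeePawns flag is on.
; With that flag off, it moves to random nearby navigable points, repeating after each successful move.
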(event OnSeePawn(PawnSensing)
  (params (Pawn :type Pawn%20Object%20Reference))
  (bind _sensedpawns (Variables|Default|GetSensedPawns))
  (if (Utilities|Array|ContainsItem _sensedpawns Pawn)
    _
    (else
      (Utilities|Array|Add _sensedpawns Pawn)
      (Variables|Default|SetClosestPawn (Utilities|Array|Get(acopy) _sensedpawns))))
  (for _index (range 0 (- (Utilities|Array|Length (Variables|Default|GetSensedPawns)) 1))
    (Development|PrintString (Utilities|GetDisplayName (Utilities|Array|Get(acopy) (Variables|Default|GetSensedPawns) _index)))
    (if (< (Transformation|GetDistanceTo (Utilities|Array|Get(acopy) (Variables|Default|GetSensedPawns) _index) self) (Transformation|GetDistanceTo (Utilities|Array|Get(acopy) (Variables|Default|GetSensedPawns) _index) (Variables|Default|GetClosestPawn)))
      (Variables|Default|SetClosestPawn (Utilities|Array|Get(acopy) (Variables|Default|GetSensedPawns) _index)))))

(event Custom|AIRoam
  (Utilities|IsValid (Variables|Default|GetClosestPawn)
    (:Is%20Valid
      (if (Variables|/Script/AIModule.PawnSensingComponent|GetbSeePawns (Variables|Default|GetPawnSensing))
        (AI|Navigation|SimpleMovetoLocation (Pawn|GetController) (Transformation|GetActorLocation (Variables|Default|GetClosestPawn)))
        (Utilities|FlowControl|Delay 0.2)
        (CallFunction|AIRoam)
        (else
          (AI|AIMoveTo self (.RandomLocation (Class|NavigationSystem|GetRandomPointinNavigableRadius (Transformation|GetActorLocation) 5e+02)) 0 5.0 false
            (:OnSuccess
              (CallFunction|AIRoam))))))
    (:Is%20Not%20Valid
      (Utilities|FlowControl|Delay 0.2)
      (CallFunction|AIRoam))))

(event EventBeginPlay
  (CallFunction|AIRoam))

(event Collision|EventActorBeginOverlap
  (params (OtherActor :type Actor%20Object%20Reference)))

(event EventTick
  (params (DeltaSeconds :type Float%20%28single-precision%29)))

(fn ConstructionScript)