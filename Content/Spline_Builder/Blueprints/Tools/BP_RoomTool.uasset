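; BP_RoomTool is an editor building tool whose construction script generates a rectangular room from modular wall and corner pillar meshes.
; The lengths of two splines and the chosen mesh size set how many wall pieces fill each side.
; Four instanced wall components and one corner component receive the pieces, with toggles per wall and pillar.
; Optional dynamic plaster materials recolor exterior and interior, and a preset selection rotates the actor.
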(fn ConstructionScript
  ;[1 1 1] Setting Variables
  ;;[1 1 1] Set the size of the mesh -1
  (LocalVariables|SetWall%20Mesh%20Size%20-1 (Utilities|Select :Index (Variables|MeshSettings|GetMesh%20Size) :NewEnumerator0 99.0 :NewEnumerator1 199.0 :NewEnumerator5 399.0))
  ;;[1 1 1] Set the real size of the mesh
  (LocalVariables|SetWall%20Mesh%20Size (Utilities|Select :Index (Variables|MeshSettings|GetMesh%20Size) :NewEnumerator0 1e+02 :NewEnumerator1 2e+02 :NewEnumerator5 4e+02))
  ;;[1 1 1] Set wall static mesh
  (LocalVariables|SetWall%20Static%20Mesh (Utilities|Select :Index (Variables|MeshSettings|GetMesh%20Size) :NewEnumerator0 (Variables|MeshSettings|WallMeshes|GetWall%20100%20x%20100) :NewEnumerator1 (Variables|MeshSettings|WallMeshes|GetWall%20200%20x%20200) :NewEnumerator5 (Variables|MeshSettings|WallMeshes|GetWall%20400%20x%20400)))
  ;;[1 1 1] Set the Wall Instance Component mesh
  (Components|StaticMesh|SetStaticMesh (Variables|Default|GetCorner%20Instance%20Component) (Variables|MeshSettings|CornerMeshes|GetCorner%2025%20x%2025))
  ;;[1 1 1] Set the Wall Instance Component mesh
  (Components|StaticMesh|SetStaticMesh (Variables|Default|GetWall%20Instance%20Component%201) (LocalVariables|GetWall%20Static%20Mesh))
  ;;[1 1 1] Set the Wall Instance Component mesh
  (Components|StaticMesh|SetStaticMesh (Variables|Default|GetWall%20Instance%20Component%202) (LocalVariables|GetWall%20Static%20Mesh))
  ;;[1 1 1] Set the Wall Instance Component mesh
  (Components|StaticMesh|SetStaticMesh (Variables|Default|GetWall%20Instance%20Component%203) (LocalVariables|GetWall%20Static%20Mesh))
  ;;[1 1 1] Set the Wall Instance Component mesh
  (Components|StaticMesh|SetStaticMesh (Variables|Default|GetWall%20Instance%20Component%204) (LocalVariables|GetWall%20Static%20Mesh))
  ;;[1 1 1] Set Spline X length
  (LocalVariables|SetSpline%20X%20Length (Spline|GetSplineLength (Variables|Default|GetSpline%20X)))
  ;;[1 1 1] Set Spline Z length
  (LocalVariables|SetSpline%20Y%20Length (Spline|GetSplineLength (Variables|Default|GetSpline%20Y)))
  ;;[1 1 1] Is Spline X longer = or > then 100
  (if (>= (LocalVariables|GetSpline%20X%20Length) (LocalVariables|GetWall%20Mesh%20Size))
    ;;[1 1 1] Is Spline Y longer = or > then 100
    (if (>= (LocalVariables|GetSpline%20Y%20Length) (LocalVariables|GetWall%20Mesh%20Size))
      ;[1 1 1] Construct Walls
      ;;[1 1 1] Set number of meshes in the x meshes
      (LocalVariables|SetX%20Meshes (.ReturnValue (Math|Float|Division(WholeandRemainder) (LocalVariables|GetSpline%20X%20Length) (LocalVariables|GetWall%20Mesh%20Size%20-1))))
      ;;[1 1 1] Set number of meshes in the Y meshes
      (LocalVariables|SetY%20Meshes (.ReturnValue (Math|Float|Division(WholeandRemainder) (LocalVariables|GetSpline%20Y%20Length) (LocalVariables|GetWall%20Mesh%20Size%20-1))))
      ;;[1 1 1] For Loop number of meshes
      (for _index (range 0 (+ (LocalVariables|GetX%20Meshes) (LocalVariables|GetY%20Meshes)))
        (LocalVariables|SetLoop%20Index _index)
        ;;[1 1 1] Is X Meshes > Loop Index
        (if (> (LocalVariables|GetX%20Meshes) (LocalVariables|GetLoop%20Index))
          ;;[1 1 1] Use wall 1
          (if (Variables|MeshSettings|EditMeshes|GetUse%20Wall%201)
            ;;[1 1 1] Set wall 1 instance locations
            (Components|InstancedStaticMesh|AddInstance (Variables|Default|GetWall%20Instance%20Component%201) (Math|Transform|MakeTransform (Math|Vector|MakeVector (.Y (Math|Vector|BreakVector (Spline|GetLocationatDistanceAlongSpline (Variables|Default|GetSpline%20X) (* (LocalVariables|GetLoop%20Index) (LocalVariables|GetWall%20Mesh%20Size)) "Local"))) (+ (.X (Math|Vector|BreakVector (Spline|GetLocationatDistanceAlongSpline (Variables|Default|GetSpline%20X) (* (LocalVariables|GetLoop%20Index) (LocalVariables|GetWall%20Mesh%20Size)) "Local"))) (LocalVariables|GetWall%20Mesh%20Size)) 0.0)))
            ;;[1 1 1] Set wall 1 rotation
            (Transformation|SetRelativeRotation (Variables|Default|GetWall%20Instance%20Component%201) "0,-90.000000, 0" false false))
          ;;[1 1 1] Use wall 2
          (if (Variables|MeshSettings|EditMeshes|GetUse%20Wall%202)
            ;;[1 1 1] Set wall 2 instance locations
            (Components|InstancedStaticMesh|AddInstance (Variables|Default|GetWall%20Instance%20Component%203) (Math|Transform|MakeTransform (Math|Vector|MakeVector (- (.Y (Math|Vector|BreakVector (Spline|GetLocationatDistanceAlongSpline (Variables|Default|GetSpline%20X) (* (LocalVariables|GetLoop%20Index) (LocalVariables|GetWall%20Mesh%20Size)) "Local"))) (LocalVariables|GetSpline%20Y%20Length)) (- (+ (.X (Math|Vector|BreakVector (Spline|GetLocationatDistanceAlongSpline (Variables|Default|GetSpline%20X) (* (LocalVariables|GetLoop%20Index) (LocalVariables|GetWall%20Mesh%20Size)) "Local"))) (LocalVariables|GetWall%20Mesh%20Size)) (LocalVariables|GetSpline%20X%20Length)) 0.0) "0,0.000000, 0" "1.000000,1,1"))
            ;;[1 1 1] Set wall 2 rotation
            (Transformation|SetRelativeRotation (Variables|Default|GetWall%20Instance%20Component%203) "0,90.000000, 0" false false)))
        ;;[1 1 1] Is the Loop Index > Y Meshes
        (if (> (LocalVariables|GetY%20Meshes) (LocalVariables|GetLoop%20Index))
          ;;[1 1 1] Use wall 3
          (if (Variables|MeshSettings|EditMeshes|GetUse%20Wall%203)
            ;;[1 1 1] Set wall 3 instance locations
            (Components|InstancedStaticMesh|AddInstance (Variables|Default|GetWall%20Instance%20Component%202) (Math|Transform|MakeTransform (Math|Vector|MakeVector (.Y (Math|Vector|BreakVector (Spline|GetLocationatDistanceAlongSpline (Variables|Default|GetSpline%20Y) (* (LocalVariables|GetLoop%20Index) (LocalVariables|GetWall%20Mesh%20Size)) "Local"))) (- (+ (.X (Math|Vector|BreakVector (Spline|GetLocationatDistanceAlongSpline (Variables|Default|GetSpline%20Y) (* (LocalVariables|GetLoop%20Index) (LocalVariables|GetWall%20Mesh%20Size)) "Local"))) (LocalVariables|GetWall%20Mesh%20Size)) (LocalVariables|GetSpline%20Y%20Length)) 0.0) "0,0.000000, 0")))
          ;;[1 1 1] Use Wall 4
          (if (Variables|MeshSettings|EditMeshes|GetUse%20Wall%204)
            ;;[1 1 1] Set wall 4 instance locations
            (Components|InstancedStaticMesh|AddInstance (Variables|Default|GetWall%20Instance%20Component%204) (Math|Transform|MakeTransform (Math|Vector|MakeVector (- (.Y (Math|Vector|BreakVector (Spline|GetLocationatDistanceAlongSpline (Variables|Default|GetSpline%20Y) (* (LocalVariables|GetLoop%20Index) (LocalVariables|GetWall%20Mesh%20Size)) "Local"))) (LocalVariables|GetSpline%20X%20Length)) (+ (.X (Math|Vector|BreakVector (Spline|GetLocationatDistanceAlongSpline (Variables|Default|GetSpline%20Y) (* (LocalVariables|GetLoop%20Index) (LocalVariables|GetWall%20Mesh%20Size)) "Local"))) (LocalVariables|GetWall%20Mesh%20Size)) 0.0) "0,0.000000, 0"))
            ;;[1 1 1] Set wall 4 rotation
            (Transformation|SetRelativeRotation (Variables|Default|GetWall%20Instance%20Component%204) "0,180.000000, 0" false false)))
        ;;[1 1 1] Is the Loop Index = 0
        (if (== (LocalVariables|GetLoop%20Index) 0)
          ;;[1 1 1] Use piller 1
          (if (Variables|MeshSettings|EditMeshes|GetUse%20Piller%201)
            ;;[1 1 1] Add corner instance at location
            (Components|InstancedStaticMesh|AddInstance (Variables|Default|GetCorner%20Instance%20Component) (Math|Transform|MakeTransform "0,25.000000,0.000000" "0,0.000000, 0")))
          ;;[1 1 1] Use piller 2
          (if (Variables|MeshSettings|EditMeshes|GetUse%20Piller%202)
            ;;[1 1 1] Add corner instance at location
            (Components|InstancedStaticMesh|AddInstance (Variables|Default|GetCorner%20Instance%20Component) (Math|Transform|MakeTransform (Math|Vector|MakeVector (+ (LocalVariables|GetSpline%20X%20Length) 25.0) 25.0 0.0) "0,0.000000, 0")))
          ;;[1 1 1] Use piller 3
          (if (Variables|MeshSettings|EditMeshes|GetUse%20Piller%203)
            ;;[1 1 1] Add corner instance at location
            (Components|InstancedStaticMesh|AddInstance (Variables|Default|GetCorner%20Instance%20Component) (Math|Transform|MakeTransform (Math|Vector|MakeVector 0.0 (* (+ (LocalVariables|GetSpline%20Y%20Length) 0.0) -1.0) 0.0) "0,0.000000, 0")))
          ;;[1 1 1] Use piller 4
          (if (Variables|MeshSettings|EditMeshes|GetUse%20Piller%204)
            ;;[1 1 1] Add corner instance at location
            (Components|InstancedStaticMesh|AddInstance (Variables|Default|GetCorner%20Instance%20Component) (Math|Transform|MakeTransform (Math|Vector|MakeVector (+ (LocalVariables|GetSpline%20X%20Length) 25.0) (* (+ (LocalVariables|GetSpline%20Y%20Length) 0.0) -1.0) 0.0) "0,0.000000, 0")))))
      ;;[1 1 1] Set materials colors
      (if (Variables|MeshSettings|EditColor|GetEdit%20Exterior%20Paint%20Color)
        (bind _returnvalue (Rendering|Material|CreateDynamicMaterialInstance (Variables|Default|GetWall%20Instance%20Component%201) 0 "/Game/Spline_Builder/Materials/M_Plaster.M_Plaster" :!class /Script/Engine.PrimitiveComponent))
        (Rendering|Material|SetMaterial (Variables|Default|GetWall%20Instance%20Component%202) 0 _returnvalue)
        (Rendering|Material|SetVectorParameterValue :self _returnvalue :ParameterName "Color" :!class /Script/Engine.MaterialInstanceDynamic))
      (if (Variables|MeshSettings|EditColor|GetEdit%20Interior%20Paint%20Color)
        (bind _returnvalue_2 (Rendering|Material|CreateDynamicMaterialInstance (Variables|Default|GetWall%20Instance%20Component%201) 2 "/Game/Spline_Builder/Materials/M_Plaster.M_Plaster" :!class /Script/Engine.PrimitiveComponent))
        (Rendering|Material|SetMaterial (Variables|Default|GetWall%20Instance%20Component%202) 2 _returnvalue_2)
        (Rendering|Material|SetVectorParameterValue :self _returnvalue_2 :ParameterName "Color" :!class /Script/Engine.MaterialInstanceDynamic))
      ;;[1 1 1] Rotation
      (if (not (== (Variables|MeshSettings|GetActor%20Rotation) (LocalVariables|GetSelected%20Rotation)))
        (Transformation|SetActorRotation (Utilities|Select :Index (Variables|MeshSettings|GetActor%20Rotation) :NewEnumerator0 "0,0.000000,0" :NewEnumerator1 "0.000000,90.000000,0.000000" :NewEnumerator5 "0.000000,180.000000,0" :NewEnumerator6 "0.000000,270.000000,0.000000" :NewEnumerator7 "0.000000,360.000000,0.000000"))
        (LocalVariables|SetSelected%20Rotation (Variables|MeshSettings|GetActor%20Rotation))))))