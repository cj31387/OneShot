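; Construction-script wall builder tool that tiles a wall mesh in a grid sized by two splines.
; SplineX length sets the column count and SplineZ length the rows, using the selected mesh size and full or half height.
; A single loop wraps column and row indices to place pieces on an instanced mesh component.
; It optionally tints plaster materials through dynamic instances and snaps actor yaw to preset right angles.
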(fn ConstructionScript
  ;[1 1 1] Setting Variables
  ;;[1 1 1] Set the high of the the meshes full size and half size used when using half meshes
  (LocalVariables|SetWall%20Mesh%20High (select (Variables|MeshSettings|GetHalf%20Hight) 162.5 325.0))
  ;;[1 1 1] Set the size of the mesh -1
  (LocalVariables|SetWall%20Mesh%20Size%20-1 (Utilities|Select :Index (Variables|MeshSettings|GetMesh%20Size) :NewEnumerator0 99.0 :NewEnumerator1 199.0 :NewEnumerator5 399.0))
  ;;[1 1 1] Set the real size of the mesh
  (LocalVariables|SetWall%20Mesh%20Size (Utilities|Select :Index (Variables|MeshSettings|GetMesh%20Size) :NewEnumerator0 1e+02 :NewEnumerator1 2e+02 :NewEnumerator5 4e+02))
  ;;[1 1 1] Set wall static mesh
  (LocalVariables|SetWall%20Static%20Mesh (Utilities|Select :Index (Variables|MeshSettings|GetMesh%20Size) :NewEnumerator0 (Variables|MeshSettings|WallMeshes|GetWall%20100%20x%20100) :NewEnumerator1 (Variables|MeshSettings|WallMeshes|GetWall%20200%20x%20200) :NewEnumerator5 (Variables|MeshSettings|WallMeshes|GetWall%20400%20x%20400)))
  ;;[1 1 1] Set the Wall Instance Component mesh
  (Components|StaticMesh|SetStaticMesh (Variables|Default|GetWall%20Instance%20Component) (LocalVariables|GetWall%20Static%20Mesh))
  ;;[1 1 1] Set Spline X length
  (LocalVariables|SetSpline%20X%20Length (Spline|GetSplineLength (Variables|Default|GetSpline%20X)))
  ;;[1 1 1] Set Spline Z length
  (LocalVariables|SetSpline%20Z%20Length (Spline|GetSplineLength (Variables|Default|GetSpline%20Z)))
  ;;[1 1 1] Is Spline X longer = or > then 100
  (if (>= (LocalVariables|GetSpline%20X%20Length) (LocalVariables|GetWall%20Mesh%20Size))
    ;[1 1 1] Wall Construction
    ;;[1 1 1] Get how many meshes will fit along the X & Z splines
    (LocalVariables|SetX%20Meshes (.ReturnValue (Math|Float|Division(WholeandRemainder) (LocalVariables|GetSpline%20X%20Length) (LocalVariables|GetWall%20Mesh%20Size%20-1))))
    (LocalVariables|SetZ%20Meshes (- (.ReturnValue (Math|Float|Division(WholeandRemainder) (LocalVariables|GetSpline%20Z%20Length) (LocalVariables|GetWall%20Mesh%20High))) 1))
    ;;[1 1 1] For Loop
    (for _index (range 0 (* (.ReturnValue (Math|Float|Division(WholeandRemainder) (LocalVariables|GetSpline%20X%20Length) (LocalVariables|GetWall%20Mesh%20Size%20-1))) (Math|Integer|SelectInt 1 (.ReturnValue (Math|Float|Division(WholeandRemainder) (LocalVariables|GetSpline%20Z%20Length) (LocalVariables|GetWall%20Mesh%20High))) (== (.ReturnValue (Math|Float|Division(WholeandRemainder) (LocalVariables|GetSpline%20Z%20Length) (LocalVariables|GetWall%20Mesh%20High))) 0))))
      ;;[1 1 1] Add 1 to the Exec Index every loop
      (LocalVariables|SetExec%20Index (+ (LocalVariables|GetExec%20Index) 1))
      ;;[1 1 1] Is Exec = X Meshes
      (if (== (LocalVariables|GetExec%20Index) (LocalVariables|GetX%20Meshes))
        ;;[1 1 1] Set new High Index and set Exec Index
        (LocalVariables|SetHight%20Index (Math|Integer|SelectInt (Math|Integer|SelectInt (LocalVariables|GetZ%20Meshes) 0 (> (LocalVariables|GetZ%20Meshes) 0)) (+ (LocalVariables|GetHight%20Index) 1) (> (+ (LocalVariables|GetHight%20Index) 1) (LocalVariables|GetZ%20Meshes))))
        (LocalVariables|SetExec%20Index 0))
      ;;[1 1 1] Add instance at the transform
      (Components|InstancedStaticMesh|AddInstance (Variables|Default|GetWall%20Instance%20Component) (Math|Transform|MakeTransform (Math|Vector|MakeVector (.Y (Math|Vector|BreakVector (Spline|GetLocationatDistanceAlongSpline (Variables|Default|GetSpline%20X) (* (LocalVariables|GetExec%20Index) (LocalVariables|GetWall%20Mesh%20Size)) "Local"))) (+ (.X (Math|Vector|BreakVector (Spline|GetLocationatDistanceAlongSpline (Variables|Default|GetSpline%20X) (* (LocalVariables|GetExec%20Index) (LocalVariables|GetWall%20Mesh%20Size)) "Local"))) 1e+02) (+ (.Z (Math|Vector|BreakVector (Spline|GetLocationatDistanceAlongSpline (Variables|Default|GetSpline%20X) (* (LocalVariables|GetExec%20Index) (LocalVariables|GetWall%20Mesh%20Size)) "Local"))) (* (LocalVariables|GetHight%20Index) (LocalVariables|GetWall%20Mesh%20High)))) "0,0.000000, 0"))
      ;;[1 1 1] Set Interior Wall Color
      (if (Variables|MeshSettings|ColorSettings|GetEdit%20Interior%20Wall%20Color)
        (for (_array_element _array_index) (Rendering|Material|GetMaterials (Variables|Default|GetWall%20Instance%20Component))
          (if (== _array_element "/Game/Spline_Builder/Materials/M_Plaster.M_Plaster")
            (bind _returnvalue (Rendering|Material|CreateDynamicMaterialInstance (Variables|Default|GetWall%20Instance%20Component) _array_index 0 :!class /Script/Engine.PrimitiveComponent))
            (Rendering|Material|SetVectorParameterValue _returnvalue "Color" (Variables|MeshSettings|ColorSettings|GetInterior%20Wall%20Color) :!class /Script/Engine.MaterialInstanceDynamic)))))
    ;;[1 1 1] Rotation
    (if (not (== (Variables|MeshSettings|GetActor%20Rotation) (LocalVariables|GetSelected%20Rotation)))
      (Transformation|SetActorRotation (Utilities|Select :Index (Variables|MeshSettings|GetActor%20Rotation) :NewEnumerator0 "0,0.000000,0" :NewEnumerator1 "0.000000,90.000000,0.000000" :NewEnumerator5 "0.000000,180.000000,0" :NewEnumerator6 "0.000000,270.000000,0.000000" :NewEnumerator7 "0.000000,360.000000,0.000000"))
      (LocalVariables|SetSelected%20Rotation (Variables|MeshSettings|GetActor%20Rotation)))))