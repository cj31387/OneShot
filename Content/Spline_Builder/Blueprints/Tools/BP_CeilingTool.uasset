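; BP_CeilingTool is a construction-script builder tool that tiles a ceiling grid from instanced static meshes.
; MeshSize picks the tile mesh and spacing, and the SplineX and SplineY lengths set column and row counts, dividing by slightly under tile size.
; One loop places instances row by row, sampling positions along SplineX only.
; It can tint the ceiling through a dynamic material and snap actor yaw to quarter turns.
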(fn ConstructionScript
  ;[1 1 1] Setting Variables
  ;;[1 1 1] Set the size of the mesh -1
  (LocalVariables|SetWall%20Mesh%20Size%20-1 (Utilities|Select :Index (Variables|MeshSettings|GetMesh%20Size) :NewEnumerator0 99.0 :NewEnumerator1 199.0 :NewEnumerator5 399.0))
  ;;[1 1 1] Set the real size of the mesh
  (LocalVariables|SetWall%20Mesh%20Size (Utilities|Select :Index (Variables|MeshSettings|GetMesh%20Size) :NewEnumerator0 1e+02 :NewEnumerator1 2e+02 :NewEnumerator5 4e+02))
  ;;[1 1 1] Set ceiling static mesh
  (LocalVariables|SetCeiling%20Static%20Mesh (Utilities|Select :Index (Variables|MeshSettings|GetMesh%20Size) :NewEnumerator0 (Variables|MeshSettings|CeilingMeshes|GetCeiling%20100%20x%20100) :NewEnumerator1 (Variables|MeshSettings|CeilingMeshes|GetCeiling%20200%20x%20200) :NewEnumerator5 (Variables|MeshSettings|CeilingMeshes|GetCeiling%20400%20x%20400)))
  ;;[1 1 1] Set the Wall Instance Component mesh
  (Components|StaticMesh|SetStaticMesh (Variables|Default|GetCeiling%20Instance%20Component) (LocalVariables|GetCeiling%20Static%20Mesh))
  ;;[1 1 1] Set Spline X length
  (LocalVariables|SetSpline%20X%20Length (Spline|GetSplineLength (Variables|Default|GetSpline%20X)))
  ;;[1 1 1] Set Spline Z length
  (LocalVariables|SetSpline%20Y%20Length (Spline|GetSplineLength (Variables|Default|GetSpline%20Y)))
  ;;[1 1 1] Is Spline X longer = or > then 100
  (if (>= (LocalVariables|GetSpline%20X%20Length) (LocalVariables|GetWall%20Mesh%20Size))
    ;;[1 1 1] Is Spline Y longer = or > then 100
    (if (>= (LocalVariables|GetSpline%20Y%20Length) (LocalVariables|GetWall%20Mesh%20Size))
      ;[1 1 1] Construct Ceiling
      ;;[1 1 1] Set the number of meshes in the X & Y
      (LocalVariables|SetX%20Meshes (.ReturnValue (Math|Float|Division(WholeandRemainder) (LocalVariables|GetSpline%20X%20Length) (LocalVariables|GetWall%20Mesh%20Size%20-1))))
      (LocalVariables|SetY%20Meshes (.ReturnValue (Math|Float|Division(WholeandRemainder) (LocalVariables|GetSpline%20Y%20Length) (LocalVariables|GetWall%20Mesh%20Size%20-1))))
      ;;[1 1 1] For loop for the number of meshes to spawn
      (for _index (range 0 (- (* (LocalVariables|GetX%20Meshes) (LocalVariables|GetY%20Meshes)) 1))
        ;;[1 1 1] If index 0 don't add to the Exec Index
        (if (== _index 0)
          _
          (else
            (LocalVariables|SetExec%20Index (+ (LocalVariables|GetExec%20Index) 1))))
        ;;[1 1 1] Is Exec = X Meshes
        (if (== (LocalVariables|GetExec%20Index) (LocalVariables|GetX%20Meshes))
          ;;[1 1 1] Set new High Index and set Exec Index
          (LocalVariables|SetExec%20Index 0)
          (LocalVariables|SetRow%20Index (+ (LocalVariables|GetRow%20Index) 1)))
        ;;[1 1 1] Add a new instance at the location
        (Components|InstancedStaticMesh|AddInstance (Variables|Default|GetCeiling%20Instance%20Component) (Math|Transform|MakeTransform (Math|Vector|MakeVector (+ (.X (Math|Vector|BreakVector (Spline|GetLocationatDistanceAlongSpline (Variables|Default|GetSpline%20X) (* (LocalVariables|GetExec%20Index) (LocalVariables|GetWall%20Mesh%20Size)) "Local"))) (LocalVariables|GetWall%20Mesh%20Size)) (+ (+ (* (LocalVariables|GetRow%20Index) (LocalVariables|GetWall%20Mesh%20Size)) (.Y (Math|Vector|BreakVector (Spline|GetLocationatDistanceAlongSpline (Variables|Default|GetSpline%20X) (* (LocalVariables|GetExec%20Index) (LocalVariables|GetWall%20Mesh%20Size)) "Local")))) (LocalVariables|GetWall%20Mesh%20Size)) (.Z (Math|Vector|BreakVector (Spline|GetLocationatDistanceAlongSpline (Variables|Default|GetSpline%20X) (* (LocalVariables|GetExec%20Index) (LocalVariables|GetWall%20Mesh%20Size)) "Local")))))))
      ;;[1 1 1] Edit Ceiling Color
      (if (Variables|MeshSettings|EditColor|GetEdit%20Ceiling%20Color)
        (bind _returnvalue (Rendering|Material|CreateDynamicMaterialInstance (Variables|Default|GetCeiling%20Instance%20Component) 0 0 :!class /Script/Engine.PrimitiveComponent))
        (Rendering|Material|SetMaterial (Variables|Default|GetCeiling%20Instance%20Component) 0 _returnvalue)
        (Rendering|Material|SetVectorParameterValue _returnvalue "Color" (Variables|MeshSettings|EditColor|GetCeiling%20Color) :!class /Script/Engine.MaterialInstanceDynamic))
      ;;[1 1 1] Rotation
      (if (not (== (Variables|MeshSettings|GetActor%20Rotation) (LocalVariables|GetSelected%20Rotation)))
        (Transformation|SetActorRotation (Utilities|Select :Index (Variables|MeshSettings|GetActor%20Rotation) :NewEnumerator0 "0,0.000000,0" :NewEnumerator1 "0.000000,90.000000,0.000000" :NewEnumerator5 "0.000000,180.000000,0" :NewEnumerator6 "0.000000,270.000000,0.000000" :NewEnumerator7 "0.000000,360.000000,0.000000"))
        (LocalVariables|SetSelected%20Rotation (Variables|MeshSettings|GetActor%20Rotation))))))