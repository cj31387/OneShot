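; Editor building tool that procedurally assembles a multi-storey modular box building from X, Y and Z spline lengths in its Construction Script.
; Mesh size picks the wall and floor/ceiling meshes and sets tile counts, with storeys at a fixed 325-unit height.
; Index-driven loops add instanced walls and floor/ceiling tiles, plus static mesh corner pillars, with per-side toggles.
; Dynamic materials apply optional paint, carpet and ceiling colors, then preset actor rotation is applied.
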(fn ConstructionScript
  ;[1 1 1] Setting Variables
  ;;[1 1 1] Set wall static mesh
  (LocalVariables|SetMid%20Static%20Mesh (select (and (Variables|BuildingSettings|EditMeshes|GetUse%20Ceiling) (Variables|BuildingSettings|EditMeshes|GetUse%20Floor)) (Utilities|Select :Index (Variables|BuildingSettings|GetMesh%20Size) :NewEnumerator0 (Variables|BuildingSettings|MidMeshes|GetMid%20100%20x%20100) :NewEnumerator1 (Variables|BuildingSettings|MidMeshes|GetMid%20200%20x%20200) :NewEnumerator5 (Variables|BuildingSettings|MidMeshes|GetMid%20400%20x%20400)) (select (Variables|BuildingSettings|EditMeshes|GetUse%20Floor) (Utilities|Select :Index (Variables|BuildingSettings|GetMesh%20Size) :NewEnumerator0 (Variables|BuildingSettings|FloorMeshes|GetFloor%20100%20x%20100) :NewEnumerator1 (Variables|BuildingSettings|FloorMeshes|GetFloor%20200%20x%20200) :NewEnumerator5 (Variables|BuildingSettings|FloorMeshes|GetFloor%20400%20x%20400)) (select (Variables|BuildingSettings|EditMeshes|GetUse%20Ceiling) (Utilities|Select :Index (Variables|BuildingSettings|GetMesh%20Size) :NewEnumerator0 (Variables|BuildingSettings|CeilingMeshes|GetCeiling%20100%20x%20100) :NewEnumerator1 (Variables|BuildingSettings|CeilingMeshes|GetCeiling%20200%20x%20200) :NewEnumerator5 (Variables|BuildingSettings|CeilingMeshes|GetCeiling%20400%20x%20400)) 0))))
  ;;[1 1 1] Set the Wall Instance Component mesh
  (Components|StaticMesh|SetStaticMesh (Variables|Default|GetMid%20Instance%20Component) (LocalVariables|GetMid%20Static%20Mesh))
  ;;[1 1 1] Set the size of the mesh -1
  (LocalVariables|SetMesh%20Size%20-1 (Utilities|Select :Index (Variables|BuildingSettings|GetMesh%20Size) :NewEnumerator0 99.0 :NewEnumerator1 199.0 :NewEnumerator5 399.0))
  ;;[1 1 1] Set the real size of the mesh
  (LocalVariables|SetMesh%20Size%20Float (Utilities|Select :Index (Variables|BuildingSettings|GetMesh%20Size) :NewEnumerator0 1e+02 :NewEnumerator1 2e+02 :NewEnumerator5 4e+02))
  ;;[1 1 1] Set wall static mesh
  (LocalVariables|SetWall%20Static%20Mesh (Utilities|Select :Index (Variables|BuildingSettings|GetMesh%20Size) :NewEnumerator0 (Variables|BuildingSettings|WallMeshes|GetWall%20100%20x%20100) :NewEnumerator1 (Variables|BuildingSettings|WallMeshes|GetWall%20200%20x%20200) :NewEnumerator5 (Variables|BuildingSettings|WallMeshes|GetWall%20400%20x%20400)))
  ;;[1 1 1] Set the Wall Instance Component mesh
  (Components|StaticMesh|SetStaticMesh (Variables|Default|GetWall%20Instance%20Component%201) (LocalVariables|GetWall%20Static%20Mesh))
  ;;[1 1 1] Set the Wall Instance Component mesh
  (Components|StaticMesh|SetStaticMesh (Variables|Default|GetWall%20Instance%20Component%202) (LocalVariables|GetWall%20Static%20Mesh))
  ;;[1 1 1] Set the Wall Instance Component mesh
  (Components|StaticMesh|SetStaticMesh (Variables|Default|GetWall%20Instance%20Component%203) (LocalVariables|GetWall%20Static%20Mesh))
  ;;[1 1 1] Set the Wall Instance Component mesh
  (Components|StaticMesh|SetStaticMesh (Variables|Default|GetWall%20Instance%20Component%204) (LocalVariables|GetWall%20Static%20Mesh))
  ;;[1 1 1] Set Spline X length
  (LocalVariables|SetSpline%20Z%20Length (Spline|GetSplineLength (Variables|Default|GetSpline%20Z)))
  ;;[1 1 1] Set Spline X length
  (LocalVariables|SetSpline%20X%20Length (Spline|GetSplineLength (Variables|Default|GetSpline%20X)))
  ;;[1 1 1] Set Spline Z length
  (LocalVariables|SetSpline%20Y%20Length (Spline|GetSplineLength (Variables|Default|GetSpline%20Y)))
  ;;[1 1 1] Is Spline X longer = or > then 100
  (if (> (LocalVariables|GetSpline%20Z%20Length) 0.0)
    ;;[1 1 1] Is Spline X longer = or > then 100
    (if (>= (LocalVariables|GetSpline%20X%20Length) (LocalVariables|GetMesh%20Size%20Float))
      ;;[1 1 1] Is Spline Y longer = or > then 100
      (if (>= (LocalVariables|GetSpline%20Y%20Length) (LocalVariables|GetMesh%20Size%20Float))
        ;[1 1 1] Construct Walls
        ;;[1 1 1] Set number of meshes in the x meshes
        (LocalVariables|SetX%20Meshes (.ReturnValue (Math|Float|Division(WholeandRemainder) (LocalVariables|GetSpline%20X%20Length) (LocalVariables|GetMesh%20Size%20-1))))
        ;;[1 1 1] Set number of meshes in the Y meshes
        (LocalVariables|SetY%20Meshes (.ReturnValue (Math|Float|Division(WholeandRemainder) (LocalVariables|GetSpline%20Y%20Length) (LocalVariables|GetMesh%20Size%20-1))))
        ;;[1 1 1] Set number of meshes in the Y meshes
        (LocalVariables|SetZ%20Meshes (select (== (.ReturnValue (Math|Float|Division(WholeandRemainder) (LocalVariables|GetSpline%20Z%20Length) 325.0)) 0) 1 (.ReturnValue (Math|Float|Division(WholeandRemainder) (LocalVariables|GetSpline%20Z%20Length) 325.0))))
        ;;[1 1 1] For Loop number of meshes
        (for _index (range 0 (* (+ (LocalVariables|GetX%20Meshes) (LocalVariables|GetY%20Meshes)) (LocalVariables|GetZ%20Meshes)))
          (bind _output_get (LocalVariables|SetLoop%20Index _index))
          ;;[1 1 1] If index 0 don't add to the Exec Index
          (if (== _output_get 0)
            _
            (else
              (LocalVariables|SetExec%20Index (+ (LocalVariables|GetExec%20Index) 1))))
          ;;[1 1 1] Comment
          (if (== (+ (LocalVariables|GetX%20Meshes) (LocalVariables|GetY%20Meshes)) (LocalVariables|GetExec%20Index))
            ;;[1 1 1] Set new High Index and set Exec Index
            (LocalVariables|SetExec%20Index 0)
            (if (> (- (LocalVariables|GetZ%20Meshes) 1) (LocalVariables|GetHight%20Index))
              (LocalVariables|SetHight%20Index (+ (LocalVariables|GetHight%20Index) 1))
              ;;[1 1 1] Is X Meshes > Loop Index
              (if (> (LocalVariables|GetX%20Meshes) (LocalVariables|GetExec%20Index)) :!label _label
                ;;[1 1 1] Use wall 1
                (if (Variables|BuildingSettings|EditMeshes|GetUse%20Wall%201)
                  ;;[1 1 1] Set wall 1 instance locations
                  (Components|InstancedStaticMesh|AddInstance (Variables|Default|GetWall%20Instance%20Component%201) (Math|Transform|MakeTransform (Math|Vector|MakeVector (+ (+ (.Y (Math|Vector|BreakVector (Spline|GetLocationatDistanceAlongSpline (Variables|Default|GetSpline%20X) (* (LocalVariables|GetExec%20Index) (LocalVariables|GetMesh%20Size%20Float)) "Local"))) (LocalVariables|GetSpline%20Y%20Length)) 25.0) (+ (.X (Math|Vector|BreakVector (Spline|GetLocationatDistanceAlongSpline (Variables|Default|GetSpline%20X) (* (LocalVariables|GetExec%20Index) (LocalVariables|GetMesh%20Size%20Float)) "Local"))) (LocalVariables|GetMesh%20Size%20Float)) (+ (.Z (Math|Vector|BreakVector (Spline|GetLocationatDistanceAlongSpline (Variables|Default|GetSpline%20X) (* (LocalVariables|GetExec%20Index) (LocalVariables|GetMesh%20Size%20Float)) "Local"))) (* 325.0 (Math|Conversions|ToFloat(Integer) (LocalVariables|GetHight%20Index))))) "0,0.000000, 0" "1.000000,1,1"))
                  ;;[1 1 1] Set wall 1 rotation
                  (Transformation|SetRelativeRotation (Variables|Default|GetWall%20Instance%20Component%201) "0,-90.000000, 0" false false))
                ;;[1 1 1] Use wall 2
                (if (Variables|BuildingSettings|EditMeshes|GetUse%20Wall%202)
                  ;;[1 1 1] Set wall 2 instance locations
                  (Components|InstancedStaticMesh|AddInstance (Variables|Default|GetWall%20Instance%20Component%203) (Math|Transform|MakeTransform (Math|Vector|MakeVector (+ (.Y (Math|Vector|BreakVector (Spline|GetLocationatDistanceAlongSpline (Variables|Default|GetSpline%20X) (* (LocalVariables|GetExec%20Index) (LocalVariables|GetMesh%20Size%20Float)) "Local"))) 25.0) (- (+ (.X (Math|Vector|BreakVector (Spline|GetLocationatDistanceAlongSpline (Variables|Default|GetSpline%20X) (* (LocalVariables|GetExec%20Index) (LocalVariables|GetMesh%20Size%20Float)) "Local"))) (LocalVariables|GetMesh%20Size%20Float)) (LocalVariables|GetSpline%20X%20Length)) (+ (.Z (Math|Vector|BreakVector (Spline|GetLocationatDistanceAlongSpline (Variables|Default|GetSpline%20X) (* (LocalVariables|GetExec%20Index) (LocalVariables|GetMesh%20Size%20Float)) "Local"))) (* 325.0 (Math|Conversions|ToFloat(Integer) (LocalVariables|GetHight%20Index)))))))
                  ;;[1 1 1] Set wall 2 rotation
                  (Transformation|SetRelativeRotation (Variables|Default|GetWall%20Instance%20Component%203) "0,90.000000, 0" false false)))
              ;;[1 1 1] Is the Loop Index > Y Meshes
              (if (> (LocalVariables|GetY%20Meshes) (LocalVariables|GetExec%20Index))
                ;;[1 1 1] Use wall 3
                (if (Variables|BuildingSettings|EditMeshes|GetUse%20Wall%203)
                  ;;[1 1 1] Set wall 3 instance locations
                  (Components|InstancedStaticMesh|AddInstance (Variables|Default|GetWall%20Instance%20Component%202) (Math|Transform|MakeTransform (Math|Vector|MakeVector (+ (+ (.Y (Math|Vector|BreakVector (Spline|GetLocationatDistanceAlongSpline (Variables|Default|GetSpline%20Y) (* (LocalVariables|GetExec%20Index) (LocalVariables|GetMesh%20Size%20Float)) "Local"))) (LocalVariables|GetSpline%20X%20Length)) 25.0) (- (+ (.X (Math|Vector|BreakVector (Spline|GetLocationatDistanceAlongSpline (Variables|Default|GetSpline%20Y) (* (LocalVariables|GetExec%20Index) (LocalVariables|GetMesh%20Size%20Float)) "Local"))) (LocalVariables|GetMesh%20Size%20Float)) (LocalVariables|GetSpline%20Y%20Length)) (+ (.Z (Math|Vector|BreakVector (Spline|GetLocationatDistanceAlongSpline (Variables|Default|GetSpline%20Y) (* (LocalVariables|GetExec%20Index) (LocalVariables|GetMesh%20Size%20Float)) "Local"))) (* 325.0 (Math|Conversions|ToFloat(Integer) (LocalVariables|GetHight%20Index))))) "0,0.000000, 0")))
                ;;[1 1 1] Use Wall 4
                (if (Variables|BuildingSettings|EditMeshes|GetUse%20Wall%204)
                  ;;[1 1 1] Set wall 4 instance locations
                  (Components|InstancedStaticMesh|AddInstance (Variables|Default|GetWall%20Instance%20Component%204) (Math|Transform|MakeTransform (Math|Vector|MakeVector (+ (.Y (Math|Vector|BreakVector (Spline|GetLocationatDistanceAlongSpline (Variables|Default|GetSpline%20Y) (* (LocalVariables|GetExec%20Index) (LocalVariables|GetMesh%20Size%20Float)) "Local"))) 25.0) (+ (.X (Math|Vector|BreakVector (Spline|GetLocationatDistanceAlongSpline (Variables|Default|GetSpline%20Y) (* (LocalVariables|GetExec%20Index) (LocalVariables|GetMesh%20Size%20Float)) "Local"))) (LocalVariables|GetMesh%20Size%20Float)) (+ (.Z (Math|Vector|BreakVector (Spline|GetLocationatDistanceAlongSpline (Variables|Default|GetSpline%20Y) (* (LocalVariables|GetExec%20Index) (LocalVariables|GetMesh%20Size%20Float)) "Local"))) (* 325.0 (Math|Conversions|ToFloat(Integer) (LocalVariables|GetHight%20Index))))) "0,0.000000, 0"))
                  ;;[1 1 1] Set wall 4 rotation
                  (Transformation|SetRelativeRotation (Variables|Default|GetWall%20Instance%20Component%204) "0,180.000000, 0" false false)))
              ;;[1 1 1] Is the Loop Index = 0
              (if (>= (LocalVariables|GetHight%20Index) (LocalVariables|GetExec%20Index))
                ;;[1 1 1] Use piller 1
                (if (Variables|BuildingSettings|EditMeshes|GetUse%20Piller%201)
                  ;;[1 1 1] Add corner instance at location
                  (bind _returnvalue (AddComponent|AddStaticMeshComponent false (Math|Transform|MakeTransform (Math|Vector|MakeVector -25.0 25.0 (* (LocalVariables|GetHight%20Index) 325.0)) "0.000000,90.000000, 0")))
                  (bind _output_get_2 (LocalVariables|SetCorner%201 _returnvalue))
                  (Components|StaticMesh|SetStaticMesh _output_get_2 (Variables|BuildingSettings|CornerMeshes|GetCorner%2025%20x%2025)))
                ;;[1 1 1] Use piller 2
                (if (Variables|BuildingSettings|EditMeshes|GetUse%20Piller%202)
                  ;;[1 1 1] Add corner instance at location
                  (bind _returnvalue_2 (AddComponent|AddStaticMeshComponent false (Math|Transform|MakeTransform (Math|Vector|MakeVector (+ (LocalVariables|GetSpline%20X%20Length) 25.0) 25.0 (* (LocalVariables|GetHight%20Index) 325.0)) "0,0.000000, 0")))
                  (bind _output_get_3 (LocalVariables|SetCorner%202 _returnvalue_2))
                  (Components|StaticMesh|SetStaticMesh _output_get_3 (Variables|BuildingSettings|CornerMeshes|GetCorner%2025%20x%2025)))
                ;;[1 1 1] Use piller 3
                (if (Variables|BuildingSettings|EditMeshes|GetUse%20Piller%203)
                  ;;[1 1 1] Add corner instance at location
                  (bind _returnvalue_3 (AddComponent|AddStaticMeshComponent false (Math|Transform|MakeTransform (Math|Vector|MakeVector -25.0 (* (+ (LocalVariables|GetSpline%20Y%20Length) 25.0) -1.0) (* (LocalVariables|GetHight%20Index) 325.0)) "0,180.000000, 0")))
                  (bind _output_get_4 (LocalVariables|SetCorner%203 _returnvalue_3))
                  (Components|StaticMesh|SetStaticMesh _output_get_4 (Variables|BuildingSettings|CornerMeshes|GetCorner%2025%20x%2025)))
                ;;[1 1 1] Use piller 4
                (if (Variables|BuildingSettings|EditMeshes|GetUse%20Piller%204)
                  ;;[1 1 1] Add corner instance at location
                  (bind _returnvalue_4 (AddComponent|AddStaticMeshComponent false (Math|Transform|MakeTransform (Math|Vector|MakeVector (+ (LocalVariables|GetSpline%20X%20Length) 25.0) (* (+ (LocalVariables|GetSpline%20Y%20Length) 25.0) -1.0) (* (LocalVariables|GetHight%20Index) 325.0)) "0,-90.000000, 0")))
                  (bind _output_get_5 (LocalVariables|SetCorner%204 _returnvalue_4))
                  (Components|StaticMesh|SetStaticMesh _output_get_5 (Variables|BuildingSettings|CornerMeshes|GetCorner%2025%20x%2025)))))
            (else
              (goto _label))))
        ;[1 1 1] Construct Mid
        ;;[1 1 1] Check if needed
        (if (or (Variables|BuildingSettings|EditMeshes|GetUse%20Ceiling) (Variables|BuildingSettings|EditMeshes|GetUse%20Floor))
          ;;[1 1 1] For loop for the number of meshes to spawn
          (LocalVariables|SetHight%20Index 0)
          (LocalVariables|SetExec%20Index 0)
          (for _index_2 (range 0 (- (* (* (LocalVariables|GetX%20Meshes) (LocalVariables|GetY%20Meshes)) (LocalVariables|GetZ%20Meshes)) 1))
            ;;[1 1 1] If index 0 don't add to the Exec Index
            (if (== _index_2 0)
              _
              (else
                (LocalVariables|SetExec%20Index (+ (LocalVariables|GetExec%20Index) 1))
                (LocalVariables|SetTotal%20Exec (+ (LocalVariables|GetTotal%20Exec) 1))))
            ;;[1 1 1] Is Exec = X Meshes
            (if (== (LocalVariables|GetExec%20Index) (LocalVariables|GetX%20Meshes))
              ;;[1 1 1] Set new High Index and set Exec Index
              (LocalVariables|SetExec%20Index 0)
              (LocalVariables|SetRow%20Index (+ (LocalVariables|GetRow%20Index) 1)))
            ;;[1 1 1] Check to see if we need a new hight level yet
            (if (== (LocalVariables|GetTotal%20Exec) (* (LocalVariables|GetX%20Meshes) (LocalVariables|GetY%20Meshes)))
              ;;[1 1 1] If true reset the total exec and row index for the new level and add 1 to the hight index
              (LocalVariables|SetTotal%20Exec 0)
              (LocalVariables|SetRow%20Index 0)
              (if (> (- (LocalVariables|GetZ%20Meshes) 1) (LocalVariables|GetHight%20Index))
                (LocalVariables|SetHight%20Index (+ (LocalVariables|GetHight%20Index) 1))
                ;;[1 1 1] Add a new instance at the location
                (Components|InstancedStaticMesh|AddInstance (Variables|Default|GetMid%20Instance%20Component) (Math|Transform|MakeTransform (Math|Vector|MakeVector (+ (.X (Math|Vector|BreakVector (Spline|GetLocationatDistanceAlongSpline (Variables|Default|GetSpline%20X) (* (LocalVariables|GetExec%20Index) (LocalVariables|GetMesh%20Size%20Float)) "Local"))) (LocalVariables|GetMesh%20Size%20Float)) (- (+ (- (.Y (Math|Vector|BreakVector (Spline|GetLocationatDistanceAlongSpline (Variables|Default|GetSpline%20X) (* (LocalVariables|GetExec%20Index) (LocalVariables|GetMesh%20Size%20Float)) "Local"))) (* (LocalVariables|GetRow%20Index) (LocalVariables|GetMesh%20Size%20Float))) (LocalVariables|GetMesh%20Size%20Float)) (Utilities|Select :Index (Variables|BuildingSettings|GetMesh%20Size) :NewEnumerator0 0.0 :NewEnumerator1 1e+02 :NewEnumerator5 3e+02)) (+ (.Z (Math|Vector|BreakVector (Spline|GetLocationatDistanceAlongSpline (Variables|Default|GetSpline%20X) (* (LocalVariables|GetExec%20Index) (LocalVariables|GetMesh%20Size%20Float)) "Local"))) (* 325.0 (Math|Conversions|ToFloat(Integer) (LocalVariables|GetHight%20Index)))))) :!label _label_2))
              (else
                (goto _label_2)))))
        ;[1 1 1] Set materials and colors
        ;;[1 1 1] Set Interior Wall Color
        (if (Variables|BuildingSettings|EditColor|GetEdit%20Interior%20Paint%20Color)
          (for (_array_element _array_index) (Rendering|Material|GetMaterials (Variables|Default|GetWall%20Instance%20Component%201))
            (if (== _array_element "/Game/Spline_Builder/Materials/M_Plaster.M_Plaster")
              (bind _returnvalue_5 (Rendering|Material|CreateDynamicMaterialInstance (Variables|Default|GetWall%20Instance%20Component%201) _array_index 0 :!class /Script/Engine.PrimitiveComponent))
              (Rendering|Material|SetMaterial (Variables|Default|GetWall%20Instance%20Component%202) _array_index _returnvalue_5)
              (Rendering|Material|SetVectorParameterValue _returnvalue_5 "Color" (Variables|BuildingSettings|EditColor|GetInterior%20Paint%20Color) :!class /Script/Engine.MaterialInstanceDynamic))))
        ;;[1 1 1] Edit Carpet Color
        (if (Variables|BuildingSettings|EditColor|GetEdit%20Carpet%20Color)
          (bind _returnvalue_6 (Rendering|Material|CreateDynamicMaterialInstance (Variables|Default|GetMid%20Instance%20Component) 1 "/Game/Spline_Builder/Materials/M_Carpet.M_Carpet" :!class /Script/Engine.PrimitiveComponent))
          (Rendering|Material|SetMaterial (Variables|Default|GetMid%20Instance%20Component) 1 _returnvalue_6)
          (Rendering|Material|SetScalarParameterValue _returnvalue_6 "Use Tint" (Math|Conversions|ToFloat(Boolean) (not (Variables|BuildingSettings|EditColor|GetEdit%20Carpet%20Color))) :!class /Script/Engine.MaterialInstanceDynamic)
          (Rendering|Material|SetVectorParameterValue _returnvalue_6 "Tint Color" (Variables|BuildingSettings|EditColor|GetCarpet%20Color) :!class /Script/Engine.MaterialInstanceDynamic))
        ;;[1 1 1] Edit Ceiling Color
        (if (Variables|BuildingSettings|EditColor|GetEdit%20Ceiling%20Color)
          (bind _returnvalue_7 (Rendering|Material|CreateDynamicMaterialInstance (Variables|Default|GetMid%20Instance%20Component) 0 0 :!class /Script/Engine.PrimitiveComponent))
          (Rendering|Material|SetMaterial (Variables|Default|GetMid%20Instance%20Component) 0 _returnvalue_7)
          (Rendering|Material|SetVectorParameterValue _returnvalue_7 "Color" (Variables|BuildingSettings|EditColor|GetCeiling%20Color) :!class /Script/Engine.MaterialInstanceDynamic))
        ;;[1 1 1] Rotation
        (if (not (== (Variables|BuildingSettings|GetActor%20Rotation) (LocalVariables|GetSelected%20Rotation)))
          (Transformation|SetActorRotation (Utilities|Select :Index (Variables|BuildingSettings|GetActor%20Rotation) :NewEnumerator0 "0,0.000000,0" :NewEnumerator1 "0.000000,90.000000,0.000000" :NewEnumerator5 "0.000000,180.000000,0" :NewEnumerator6 "0.000000,270.000000,0.000000" :NewEnumerator7 "0.000000,360.000000,0.000000"))
          (LocalVariables|SetSelected%20Rotation (Variables|BuildingSettings|GetActor%20Rotation)))))))