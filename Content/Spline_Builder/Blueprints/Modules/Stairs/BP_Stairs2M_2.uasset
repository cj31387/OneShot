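; BP_Stairs2M_2 is a stairs module for the Spline Builder, configured entirely in its construction script.
; Optional edit flags create dynamic materials on the stairs mesh to apply interior wall and floor colors.
; The floor branch sets "Use Tint" from the negated edit flag, so it is always zero there.
; A changed Rotation selection snaps the actor to quarter-turn angles and is cached in SelectedRotation.
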(event EventBeginPlay)

(event Collision|EventActorBeginOverlap
  (params (OtherActor :type Actor%20Object%20Reference)))

(event EventTick
  (params (DeltaSeconds :type Float%20%28single-precision%29)))

(fn ConstructionScript
  (Utilities|FlowControl|Sequence
    (:then_0
      ;[1 1 1] Wall Colors
      (if (Variables|Color|GetEdit%20Interior%20Wall%20Color)
        (bind _returnvalue (Rendering|Material|CreateDynamicMaterialInstance (Variables|Default|GetSM_Stairs2M_2) 1 0 :!class /Script/Engine.PrimitiveComponent))
        (Rendering|Material|SetVectorParameterValue _returnvalue "Color" (Variables|Color|GetInterior%20Wall%20Color) :!class /Script/Engine.MaterialInstanceDynamic))
      (if (Variables|Color|GetEdit%20Floor%20Color)
        (bind _returnvalue_2 (Rendering|Material|CreateDynamicMaterialInstance (Variables|Default|GetSM_Stairs2M_2) 0 0 :!class /Script/Engine.PrimitiveComponent))
        (Rendering|Material|SetScalarParameterValue _returnvalue_2 "Use Tint" (Math|Conversions|ToFloat(Boolean) (not (Variables|Color|GetEdit%20Floor%20Color))) :!class /Script/Engine.MaterialInstanceDynamic)
        (Rendering|Material|SetVectorParameterValue _returnvalue_2 "Tint Color" (Variables|Color|GetFloor%20Color) :!class /Script/Engine.MaterialInstanceDynamic)))
    (:then_1
      ;[1 1 1] Rotation
      (if (not (== (Variables|Control|GetRotation) (Variables|NonUI|GetSelected%20Rotation)))
        (Transformation|SetActorRotation (Utilities|Select :Index (Variables|Control|GetRotation) :NewEnumerator0 "0,0.000000,0" :NewEnumerator1 "0.000000,90.000000,0.000000" :NewEnumerator5 "0.000000,180.000000,0" :NewEnumerator6 "0.000000,270.000000,0.000000" :NewEnumerator7 "0.000000,360.000000,0.000000"))
        (Variables|NonUI|SetSelected%20Rotation (Variables|Control|GetRotation))))))