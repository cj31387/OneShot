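; BP_Elevator is a multi-story elevator actor with an interior that moves vertically and sliding doors on each floor.
; The construction script stacks left and right door instances per story, and a timeline slides both components apart, moving every floor's doors together.
; Up and down timelines lerp the interior one story at a time, replaying until CurrentStory reaches DesiredStory, with a moving-flag guard.
; The movement, door and story-setting chains have no triggering events connected.
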(fn ConstructionScript
  ;[0 0.3732 1] The loop: Lop as many times as the height
  (for _index (range 0 (- (Variables|Elevator|GetHowManyStoriesHigh) 1))
    ;[0 0.3732 1] Place the left side of the doors
    (Components|InstancedStaticMesh|AddInstance (Variables|Default|GetLeftDoor) (Math|Transform|MakeTransform (Math|Vector|MakeVector 6e+01 5.0 (* _index (Variables|Elevator|GetHeightOfAStroy))) "0.000000, 0, 0"))
    ;[0 0.3732 1] Place the right side of the doors
    (Components|InstancedStaticMesh|AddInstance (Variables|Default|GetRightDoor) (Math|Transform|MakeTransform (Math|Vector|MakeVector 1.3e+02 5.0 (* _index (Variables|Elevator|GetHeightOfAStroy)))))))