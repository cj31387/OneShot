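; BP_WallBuilder procedurally assembles a modular wall with optional doors and a single left or right corner.
; Its construction script loops over the segments, choosing wall, door or corner from corner settings and a door-index array.
; Math expressions compute offsets from segment length and width, and a PlaceInstance helper adds each transform to the matching instanced component.
; Right turns use separate inverted-material components for the corner and following pieces.
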(event EventBeginPlay)

(event Collision|EventActorBeginOverlap
  (params (OtherActor :type Actor%20Object%20Reference)))

(event EventTick
  (params (DeltaSeconds :type Float%20%28single-precision%29)))

(fn ConstructionScript
  (bind _length_of_segments (Variables|WallBuilder|GetLength%20of%20segments))
  (bind _length_of_segments_2 (Variables|WallBuilder|GetLength%20of%20segments))
  ;[0.185 0.185 0.185] The loop & save index to reduce complex wires
  (for _index (range 0 (Variables|WallBuilder|GetAmount%20of%20segments)) ; The main loop
    (Variables|WallBuilder|SetIndex _index)
    ;[0.185 0.185 0.185] The main logic for the loop decides which type to place
    (if (Variables|WallBuilder|GetPlace%20corner?) ; Look if it shall be a corner
      (if (< (Variables|WallBuilder|GetIndex) (Variables|WallBuilder|GetCorner%20Segment%20Number)) ; If we are under then place normal wall
        ;[0 0.3732 1] [Normal wall] The logic for the normal walls. Looks if a door shall be placed and looks in the array to see if this is a door
        (if (Variables|WallBuilder|GetPlace%20door?) :!label _label ; Look if there shall be placed a door
          (if (Utilities|Array|ContainsItem (Variables|WallBuilder|GetDoor%20Segment%20Number) (Variables|WallBuilder|GetIndex)) ; Look if this is the segment that shall be a door
            ;[0 0.3732 1] [Normal wall] Place door
            (Utilities|PlaceInstance (|((l*i)+(l/2)) (Variables|WallBuilder|GetIndex) (Variables|WallBuilder|GetLength%20of%20segments)) 0.0 0.0 0.0 1.0 1.0 1.0 (Variables|Default|GetDoor))
            (else
              ;[0 0.3732 1] [Normal wall] Place wall
              (Utilities|PlaceInstance (|((l*i)+(l/2)) (Variables|WallBuilder|GetIndex) (Variables|WallBuilder|GetLength%20of%20segments)) 0.0 0.0 0.0 1.0 1.0 1.0 (Variables|Default|GetWall) :!label _label_2)))
          (else
            (goto _label_2)))
        (elif (Variables|WallBuilder|GetCorner%20Left?) ; Decide which side to place
          ;[1 0.2279 0] [Left side] The logic for the left direction. Looks if there shall be placed a wall or a corner & if a door shall be placed
          (if (== (Variables|WallBuilder|GetIndex) (Variables|WallBuilder|GetCorner%20Segment%20Number)) ; Is this the corner?
            ;[1 0.2279 0] [Left side] Place corner
            (Utilities|PlaceInstance (|((i+1)*l) (Variables|WallBuilder|GetIndex) (Variables|WallBuilder|GetLength%20of%20segments)) 0.0 0.0 -9e+01 1.0 1.0 1.0 (Variables|Default|GetCorner))
            (elif (Variables|WallBuilder|GetPlace%20door?) ; Look if there shall be placed a door
              (if (Utilities|Array|ContainsItem (Variables|WallBuilder|GetDoor%20Segment%20Number) (Variables|WallBuilder|GetIndex)) ; Look if this is the segment that shall be a door
                ;[1 0.2279 0] [Left side] Place door
                (Utilities|PlaceInstance (|((n+1)*l) (Variables|WallBuilder|GetCorner%20Segment%20Number) (Variables|WallBuilder|GetLength%20of%20segments)) (|(x+(l/2)) (* -1 (|(((i-n)+1)*l) (Variables|WallBuilder|GetIndex) (Variables|WallBuilder|GetCorner%20Segment%20Number) _length_of_segments_2)) _length_of_segments_2) 0.0 -9e+01 1.0 1.0 1.0 (Variables|Default|GetDoor))
                (else
                  ;[1 0.2279 0] [Left side] Place wall
                  (Utilities|PlaceInstance (|((n+1)*l) (Variables|WallBuilder|GetCorner%20Segment%20Number) (Variables|WallBuilder|GetLength%20of%20segments)) (|(x+(l/2)) (* -1 (|(((i-n)+1)*l) (Variables|WallBuilder|GetIndex) (Variables|WallBuilder|GetCorner%20Segment%20Number) _length_of_segments)) _length_of_segments) 0.0 -9e+01 1.0 1.0 1.0 (Variables|Default|GetWall) :!label _label_3)))
              (else
                (goto _label_3))))
          (else
            ;[0 0.635 0.1089] [Right side] The logic for the right direction. Looks if there shall be placed a wall or a corner & if a door shall be placed
            (if (== (Variables|WallBuilder|GetIndex) (Variables|WallBuilder|GetCorner%20Segment%20Number)) ; Is this the corner?
              ;[0 0.635 0.1089] [Right side] Place corner
              (Utilities|PlaceInstance (|(((i+1)*l)+w) (Variables|WallBuilder|GetIndex) (Variables|WallBuilder|GetLength%20of%20segments) (Variables|WallBuilder|GetWidht%20of%20segments)) (* -1 (Variables|WallBuilder|GetWidht%20of%20segments)) 0.0 1.8e+02 1.0 1.0 1.0 (Variables|Default|GetCorner_InvertedMaterial))
              (elif (Variables|WallBuilder|GetPlace%20door?) ; Look if there shall be placed a door
                (if (Utilities|Array|ContainsItem (Variables|WallBuilder|GetDoor%20Segment%20Number) (Variables|WallBuilder|GetIndex)) ; Look if this is the segment that shall be a door
                  ;[0 0.635 0.1089] [Right side] Place door
                  (Utilities|PlaceInstance (|(((n*l)+l)+w) (Variables|WallBuilder|GetCorner%20Segment%20Number) (Variables|WallBuilder|GetLength%20of%20segments) (Variables|WallBuilder|GetWidht%20of%20segments)) (|(((i-n)*l)+(l/2)) (Variables|WallBuilder|GetIndex) (Variables|WallBuilder|GetCorner%20Segment%20Number) (Variables|WallBuilder|GetLength%20of%20segments)) 0.0 -9e+01 1.0 1.0 1.0 (Variables|Default|GetDoor_InvertedMaterial))
                  (else
                    ;[0 0.635 0.1089] [Right side] Place wall
                    (Utilities|PlaceInstance (|(((n*l)+l)+w) (Variables|WallBuilder|GetCorner%20Segment%20Number) (Variables|WallBuilder|GetLength%20of%20segments) (Variables|WallBuilder|GetWidht%20of%20segments)) (|(((i-n)*l)+(l/2)) (Variables|WallBuilder|GetIndex) (Variables|WallBuilder|GetCorner%20Segment%20Number) (Variables|WallBuilder|GetLength%20of%20segments)) 0.0 -9e+01 1.0 1.0 1.0 (Variables|Default|GetWall_InvertedMaterial) :!label _label_4)))
                (else
                  (goto _label_4)))))))
      (else
        (goto _label)))))